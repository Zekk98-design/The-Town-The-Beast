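; BP_PlaceholderSword is a placeholder melee weapon that damages enemies on contact.
; When its MeleeCollision component begins overlapping an actor tagged Enemy, it applies fixed damage with its owner as damage causer and prints the result.
; It then plays a sword hit sound at the collision's location, picked by GetNewRandomIndex, which stores the random index but does not prevent repeats.
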(event `self.MeleeCollision.OnComponentBeginOverlap`
  (params (OverlappedComponent :type "PrimitiveComponent Object Reference") (OtherActor :type "Actor Object Reference") (OtherComp :type "PrimitiveComponent Object Reference") (OtherBodyIndex :type Integer) (bFromSweep :type Boolean) (SweepResult :type "HitResult Structure (by ref)"))
  (if (`self.ActorHasTag` OtherActor "Enemy")
    (bind _returnvalue (`GameplayStatics.ApplyDamage` OtherActor 25.0 null (`self.GetOwner`) "/Script/Engine.DamageType"))
    (`KismetSystemLibrary.PrintString` (`KismetStringLibrary.Conv_DoubleToString` _returnvalue))
    (bind _output (`self.GetNewRandomIndex` (`self.SFX_SwordHits`))
      (:`Out`
        (`GameplayStatics.PlaySoundAtLocation` _output (`SceneComponent.K2_GetComponentLocation` (`self.MeleeCollision`)) (struct) 1.0 1.0 0.0 null null null)))))

(fn `UserConstructionScript`)