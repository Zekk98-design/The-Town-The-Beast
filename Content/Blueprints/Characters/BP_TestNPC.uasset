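; Test NPC that runs branching, data-table-driven dialogue with quest hooks and player choices.
; BeginPlay loads its DT_NPC_Dialogue row; WriteNextSentence activates or completes quests and types [NAME]-substituted text through a delayed character-loop macro.
; When ReadyForChoice is set, typing stops appending and PopulateChoiceButtons fills the player's dialogue widget with choices affordable in gold.
; A perk-based skill-check filter exists but is disconnected.
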(event `WriteNextSentence`
  (bind _dialogue_struct_sentences_array (break `/Game/Structures/Struct_Dialogue` (`self.Dialogue_Struct`)))
  (bind _dialogue_struct_sentences_array_2 (break `/Game/Structures/Struct_Dialogue` (`self.Dialogue_Struct`)))
  (bind _output_sentence_text (break `/Game/Structures/Struct_Sentence` (`|GetArrayItem` _dialogue_struct_sentences_array_2 (`self.DialogueCurrentID`))))
  (bind (_output_sentence_text_2 _output_sentence_ischoice _output_choices _output_startsquest _output_questid _output_endsdialogue _output_newbookmarkid _output_questcompleted) (break `/Game/Structures/Struct_Sentence` (`|GetArrayItem` _dialogue_struct_sentences_array (`self.DialogueCurrentID`))))
  (set `self.DialogueOutput` "")
  (`|ExecutionSequence`
    (:`then_0`
      (`PanelWidget.ClearChildren` (`/Game/Blueprints/Widgets/WBP_Dialogue.ScrollBox_81` (`/Game/Blueprints/Characters/ThirdPersonCharacter.DialogueWidget` (cast `/Game/Blueprints/Characters/ThirdPersonCharacter` (`GameplayStatics.GetPlayerCharacter` 0) :!pure true))))
      (if (`self.ReadyForChoice`)
        (`self.PopulateChoiceButtons`)))
    (:`then_1`
      (if _output_startsquest
        ;[1 1 1] Activate New Quest
        (`BlueprintMapLibrary.Map_Add` (`.QuestActivationMap_18_DC771C1246DD67AEB5581D9B6467EBA9` (break `/Game/Structures/Struct_PlayerData` (`/Game/Blueprints/GIBP_GameInstance.PlayerData` (cast `/Game/Blueprints/GIBP_GameInstance` (`GameplayStatics.GetGameInstance`) :!pure true)))) _output_questid true)))
    (:`then_2`
      (if (`KismetStringLibrary.NotEqual_StrStr` _output_questcompleted)
        (`/Game/Blueprints/GIBP_GameInstance.CompleteQuest` (cast `/Game/Blueprints/GIBP_GameInstance` (`GameplayStatics.GetGameInstance`) :!pure true) _output_questcompleted)))
    (:`then_3`
      (bind _array_element (`self.ForEachLoopWithDelay` (`KismetStringLibrary.GetCharacterArrayFromString` (`KismetStringLibrary.Replace` _output_sentence_text "[NAME]" (`.Name_3_7DDA3B5341DB2876CFB5129D03435E6B` (break `/Game/Structures/Struct_PlayerStats` (`/Game/Blueprints/GIBP_GameInstance.PlayerStats` (cast `/Game/Blueprints/GIBP_GameInstance` (`GameplayStatics.GetGameInstance`) :!pure true)))) "CaseSensitive")) (`/Game/ThirdPersonBP/Blueprints/ThirdPersonGameMode.TextDelay` (`self.GameMode`)))
        (:`Loop Body`
          (if (not (`self.ReadyForChoice`))
            (set `self.DialogueOutput` (`KismetStringLibrary.Concat_StrStr` (`self.DialogueOutput`) _array_element))))))))

(event `self.ReceiveBeginPlay`
  ;[1 1 1] Set GameMode and Dialogue Struct
  (bind _asthird_person_game_mode (cast `/Game/ThirdPersonBP/Blueprints/ThirdPersonGameMode` (`GameplayStatics.GetGameMode`)))
  (set `self.GameMode` _asthird_person_game_mode)
  (bind _outrownames (`DataTableFunctionLibrary.GetDataTableRowNames` "/Game/Structures/DT_NPC_Dialogue.DT_NPC_Dialogue"))
  (bind _returnvalue (`|GetDataTableRow` "/Game/Structures/DT_NPC_Dialogue.DT_NPC_Dialogue" (`|GetArrayItem` _outrownames (`self.DialogueStructID`)))
    (:`then`
      (set `self.Dialogue_Struct` _returnvalue))))

(event `PopulateChoiceButtons`
  (bind _dialogue_struct_sentences_array (break `/Game/Structures/Struct_Dialogue` (`self.Dialogue_Struct`)))
  (bind (_output_sentence_text _output_sentence_ischoice _output_choices) (break `/Game/Structures/Struct_Sentence` (`|GetArrayItem` _dialogue_struct_sentences_array (`self.DialogueCurrentID`))))
  ;[1 1 1] Offer Choices
  (for _array_element _output_choices
    (if (<= (`.Choice_Cost_20_C9DCFF2544DD24D2B5CBA795B1F4D520` (break `/Game/Structures/Struct_Choice` _array_element)) (`.Gold_30_5B0109C14F70D1B65D9682A489587456` (break `/Game/Structures/Struct_PlayerStats` (`/Game/Blueprints/GIBP_GameInstance.PlayerStats` (cast `/Game/Blueprints/GIBP_GameInstance` (`GameplayStatics.GetGameInstance`) :!pure true)))))
      (bind _returnvalue (`|CreateWidget` "/Game/Blueprints/Widgets/WBP_Dialogue_ChoiceButton.WBP_Dialogue_ChoiceButton_C"))
      (`|ExecutionSequence`
        (:`then_0`
          (bind (_choice_text _choice_skilltext _choice_bookmarkid _choice_skillcheck _choice_cost _choice_eventtrigger) (break `/Game/Structures/Struct_Choice` _array_element))
          (set `/Game/Blueprints/Widgets/WBP_Dialogue_ChoiceButton.Choice` _choice_text _returnvalue))
        (:`then_1`
          (set `/Game/Blueprints/Widgets/WBP_Dialogue_ChoiceButton.Reason` _choice_skilltext _returnvalue))
        (:`then_2`
          (set `/Game/Blueprints/Widgets/WBP_Dialogue_ChoiceButton.BookmarkID` _choice_bookmarkid _returnvalue))
        (:`then_3`
          (set `/Game/Blueprints/Widgets/WBP_Dialogue_ChoiceButton.CurrentNPC` self _returnvalue))
        (:`then_4`
          (set `/Game/Blueprints/Widgets/WBP_Dialogue_ChoiceButton.Cost` _choice_cost _returnvalue))
        (:`then_5`
          (set `/Game/Blueprints/Widgets/WBP_Dialogue_ChoiceButton.EventTrigger` _choice_eventtrigger _returnvalue))
        (:`then_6`
          (set `/Game/Blueprints/Widgets/WBP_Dialogue_ChoiceButton.SkillCheck` _choice_skillcheck _returnvalue)
          (`PanelWidget.AddChild` (`/Game/Blueprints/Widgets/WBP_Dialogue.ScrollBox_81` (`/Game/Blueprints/Characters/ThirdPersonCharacter.DialogueWidget` (cast `/Game/Blueprints/Characters/ThirdPersonCharacter` (`GameplayStatics.GetPlayerCharacter` 0) :!pure true))) _returnvalue))))))

(fn `UserConstructionScript`)