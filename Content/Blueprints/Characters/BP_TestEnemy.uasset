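; Test enemy character that chases the player on sight, bites at close range and rewards gold and EXP when killed.
; Pawn sensing drives an AI move toward the player, then a delayed attack sphere-traces forward, applies damage and plays a random bite sound, with a flag blocking new chases mid-attack.
; Incoming damage reduces health, and death pays a random gold amount plus EXP through the game instance before destroying the actor.
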(event `self.ReceiveAnyDamage`
  (params (Damage :type "Float (single-precision)") (DamageType :type "DamageType Object Reference") (InstigatedBy :type "Controller Object Reference") (DamageCauser :type "Actor Object Reference"))
  ;[1 1 1] Take Damage
  (set `self.Health` (- (`self.Health`) Damage))
  (if (<= (`self.Health`) 0.0)
    (`self.Die`)))

(event `self.PawnSensing.OnSeePawn`
  (params (Pawn :type "Pawn Object Reference"))
  ;[1 1 1] Chase Player
  (if (not (`self.IsMidAttack`))
    (bind _asthird_person_character (cast `/Game/Blueprints/Characters/ThirdPersonCharacter` Pawn))
    (`|AIMoveTo` self (0.0 0.0 0.0) _asthird_person_character 150.0
      (:`OnSuccess`
        (`self.Attack`)))))

(event `Attack`
  (bind _returnvalue (`self.K2_GetActorLocation`))
  ;[1 1 1] Attack
  (set `self.IsMidAttack` true)
  (`KismetSystemLibrary.Delay` 0.5)
  (`|ExecutionSequence`
    (:`then_0`
      (`self.PlayBiteSFX`)
      (bind (_outhit _returnvalue_2) (`KismetSystemLibrary.SphereTraceSingleForObjects` _returnvalue (+ _returnvalue (* (`KismetMathLibrary.GetForwardVector` (`SceneComponent.K2_GetComponentRotation` (`self.CapsuleComponent`))) (`self.AttackRange`))) 0.0 (`|MakeArray` "ObjectTypeQuery3" :!type "EObjectTypeQuery Enum")))
      (if _returnvalue_2
        (bind _asthird_person_character (cast `/Game/Blueprints/Characters/ThirdPersonCharacter` (`.HitActor` (`GameplayStatics.BreakHitResult` _outhit))))
        (`GameplayStatics.ApplyDamage` _asthird_person_character (`self.AttackDamage`))
        (`KismetSystemLibrary.PrintString` "Damaged player")))
    (:`then_1`
      (set `self.IsMidAttack` false))))

(event `Die`
  (bind _asgibp_game_instance (cast `/Game/Blueprints/GIBP_GameInstance` (`GameplayStatics.GetGameInstance`)))
  (`/Game/Blueprints/GIBP_GameInstance.GainGold` _asgibp_game_instance (`KismetMathLibrary.RandomIntegerInRange` (`self.MinGoldDrop`) (`self.MaxGoldDrop`)))
  (`/Game/Blueprints/GIBP_GameInstance.GainEXP` _asgibp_game_instance (`self.ExpDrop`))
  (`self.K2_DestroyActor`))

(event `PlayBiteSFX`
  (bind _output (`self.GetNewRandomIndex` (`self.BiteSFX`))
    (:`Out`
      (`GameplayStatics.PlaySoundAtLocation` _output (`SceneComponent.K2_GetComponentLocation` (`self.CapsuleComponent`)) (struct) 1.0 1.0 0.0 null null null))))

(fn `UserConstructionScript`)