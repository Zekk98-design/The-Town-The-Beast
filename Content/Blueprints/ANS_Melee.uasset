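; Animation notify state named "Melee Attack" that opens the sword's hit window during a melee animation.
; On begin it sets the MeleeCollision of the owning ThirdPersonCharacter's BP_PlaceholderSword to query-only, and on end it sets it back to no collision.
; The sword is found by casting the character's first child actor, so it depends on that attachment order.
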(fn `GetNotifyName`
  (returns (ReturnValue :type String))
  (return "Melee Attack"))

(fn `Received_NotifyBegin`
  (params (MeshComp :type "SkeletalMeshComponent Object Reference") (Animation :type "AnimSequenceBase Object Reference") (TotalDuration :type "Float (double-precision)"))
  (returns (ReturnValue :type Boolean))
  (`PrimitiveComponent.SetCollisionEnabled` (`/Game/Mixamo/BP_PlaceholderSword.MeleeCollision` (cast `/Game/Mixamo/BP_PlaceholderSword` (`|GetArrayItem` (`Actor.GetAllChildActors` (cast `/Game/Blueprints/ThirdPersonCharacter` (`ActorComponent.GetOwner` MeshComp) :!pure true) false)) :!pure true)) "QueryOnly")
  (return false))

(fn `Received_NotifyEnd`
  (params (MeshComp :type "SkeletalMeshComponent Object Reference") (Animation :type "AnimSequenceBase Object Reference"))
  (returns (ReturnValue :type Boolean))
  (`PrimitiveComponent.SetCollisionEnabled` (`/Game/Mixamo/BP_PlaceholderSword.MeleeCollision` (cast `/Game/Mixamo/BP_PlaceholderSword` (`|GetArrayItem` (`Actor.GetAllChildActors` (cast `/Game/Blueprints/ThirdPersonCharacter` (`ActorComponent.GetOwner` MeshComp) :!pure true) false)) :!pure true)) "NoCollision")
  (return false))