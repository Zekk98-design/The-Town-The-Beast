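; Game instance that holds the player's stats and quest data for an RPG, covering gold, EXP, levels, equipment and flowers.
; Gaining EXP past a threshold queues a pending level up to level 5, and completing a quest grants EXP.
; Weapon and shield functions update the equipment map and tell the ThirdPersonCharacter to change its visuals.
; Max armour counts worn armour pieces, doubled by a perk, and picking enough flowers advances the flower quest.
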(event `LevelUp`
  (bind _playerstats (`self.PlayerStats`))
  (bind (_name _gender _level _exp _maxhealth _currenthealth _maxmagic _currentmagic _maxarmour _currentarmour _gold _equipment _potions _pendinglevels) (break `/Game/Structures/Struct_PlayerStats` _playerstats))
  (if (< (`.Level_6_C2159DAF49B4901F5DC935BCBC439586` (break `/Game/Structures/Struct_PlayerStats` (`self.PlayerStats`))) 5)
    (`BlueprintMapLibrary.Map_Add` _pendinglevels (+ _level 1) true)
    (setmembers `/Game/Structures/Struct_PlayerStats` :`StructRef` _playerstats :`EXP` (- _exp 1000))))

(event `CalculateArmour`
  (bind _temparmourcounter (`self.TempArmourCounter`))
  (bind (_name _gender _level _exp _maxhealth _currenthealth _maxmagic _currentmagic _maxarmour _currentarmour _gold _equipment _potions _pendinglevels _perks) (break `/Game/Structures/Struct_PlayerStats` (`self.PlayerStats`)))
  (bind _returnvalue (`BlueprintSetLibrary.Set_Contains` _perks "NewEnumerator7"))
  (if (`BlueprintMapLibrary.Map_Find` _equipment "Armour")
    (`/Engine/EditorBlueprintResources/StandardMacros.IncrementInt` _temparmourcounter
      (:`  `
        (if _returnvalue
          (`/Engine/EditorBlueprintResources/StandardMacros.IncrementInt` _temparmourcounter
            (:`  `
              _))))))
  (if (`BlueprintMapLibrary.Map_Find` _equipment "Shield")
    (`/Engine/EditorBlueprintResources/StandardMacros.IncrementInt` _temparmourcounter
      (:`  `
        (if _returnvalue
          (`/Engine/EditorBlueprintResources/StandardMacros.IncrementInt` _temparmourcounter
            (:`  `
              _))))))
  (if (`BlueprintMapLibrary.Map_Find` _equipment "Helmet")
    (`/Engine/EditorBlueprintResources/StandardMacros.IncrementInt` _temparmourcounter
      (:`  `
        (if _returnvalue
          (`/Engine/EditorBlueprintResources/StandardMacros.IncrementInt` _temparmourcounter
            (:`  `
              _))))))
  (setmembers `/Game/Structures/Struct_PlayerStats` :`StructRef` (`self.PlayerStats`) :`MaxArmour` (`self.TempArmourCounter`))
  (set `self.TempArmourCounter` 0))

(fn `CompleteQuest`
  (params (`Quest ID` :type String))
  (`BlueprintMapLibrary.Map_Add` (`.QuestCompletionMap_28_4F242649420EDA3E07B31D98F37B72C1` (break `/Game/Structures/Struct_PlayerData` (`self.PlayerData`))) `Quest ID` true)
  (`self.GainEXP` 1200))

(fn `EquipFists`
  (bind (_name _gender _level _exp _maxhealth _currenthealth _maxmagic _currentmagic _maxarmour _currentarmour _gold _equipment) (break `/Game/Structures/Struct_PlayerStats` (`self.PlayerStats`)))
  (`BlueprintMapLibrary.Map_Add` _equipment "Fists" true)
  (`BlueprintMapLibrary.Map_Add` _equipment "OneHandedSword")
  (`BlueprintMapLibrary.Map_Add` _equipment "TwoHandedSword")
  (bind _asthird_person_character (cast `/Game/Blueprints/Characters/ThirdPersonCharacter` (`GameplayStatics.GetPlayerPawn` 0)))
  (`/Game/Blueprints/Characters/ThirdPersonCharacter.ActivateFists` _asthird_person_character)
  (return))

(fn `EquipOneHandedSword`
  (bind (_name _gender _level _exp _maxhealth _currenthealth _maxmagic _currentmagic _maxarmour _currentarmour _gold _equipment) (break `/Game/Structures/Struct_PlayerStats` (`self.PlayerStats`)))
  (`BlueprintMapLibrary.Map_Add` _equipment "Fists")
  (`BlueprintMapLibrary.Map_Add` _equipment "OneHandedSword" true)
  (`BlueprintMapLibrary.Map_Add` _equipment "TwoHandedSword")
  (bind _asthird_person_character (cast `/Game/Blueprints/Characters/ThirdPersonCharacter` (`GameplayStatics.GetPlayerPawn` 0)))
  (`/Game/Blueprints/Characters/ThirdPersonCharacter.ActivateOneHandedSword` _asthird_person_character)
  (return))

(fn `EquipTwoHandedSword`
  (bind (_name _gender _level _exp _maxhealth _currenthealth _maxmagic _currentmagic _maxarmour _currentarmour _gold _equipment) (break `/Game/Structures/Struct_PlayerStats` (`self.PlayerStats`)))
  (`BlueprintMapLibrary.Map_Add` _equipment "Fists")
  (`BlueprintMapLibrary.Map_Add` _equipment "OneHandedSword")
  (`BlueprintMapLibrary.Map_Add` _equipment "TwoHandedSword" true)
  (bind _asthird_person_character (cast `/Game/Blueprints/Characters/ThirdPersonCharacter` (`GameplayStatics.GetPlayerPawn` 0)))
  (`/Game/Blueprints/Characters/ThirdPersonCharacter.ActivateTwoHandedSword` _asthird_person_character)
  (return))

(fn `GainEXP`
  (params (Amount :type Integer))
  (bind _playerstats (`self.PlayerStats`))
  (setmembers `/Game/Structures/Struct_PlayerStats` :`StructRef` _playerstats :`EXP` (+ Amount (`.EXP_48_B9BE62ED4A8138BB70129AAE7A6A8CED` (break `/Game/Structures/Struct_PlayerStats` _playerstats))))
  (if (>= (`.EXP_48_B9BE62ED4A8138BB70129AAE7A6A8CED` (break `/Game/Structures/Struct_PlayerStats` (`self.PlayerStats`))) 1000)
    (`self.LevelUp`))
  (return))

(fn `GainGold`
  (params (Amount :type Integer))
  (bind _playerstats (`self.PlayerStats`))
  (setmembers `/Game/Structures/Struct_PlayerStats` :`StructRef` _playerstats :`Gold` (+ Amount (`.Gold_30_5B0109C14F70D1B65D9682A489587456` (break `/Game/Structures/Struct_PlayerStats` _playerstats))))
  (return))

(fn `LoseGold`
  (params (Amount :type Integer))
  (bind _playerstats (`self.PlayerStats`))
  (setmembers `/Game/Structures/Struct_PlayerStats` :`StructRef` _playerstats :`Gold` (- (`.Gold_30_5B0109C14F70D1B65D9682A489587456` (break `/Game/Structures/Struct_PlayerStats` _playerstats)) Amount))
  (return))

(fn `PickFlower`
  (params (Colour :type "/Game/Structures/ENUM_FlowerColour Enum" :default "NewEnumerator0"))
  (bind ((`BlueFlowerCount_5_425584AE400571B6487B78B53038016C` _blueflowercount) (`YellowFlowerCount_8_6600622242C7917FE03DBF9DE3E33EB4` _yellowflowercount) (`RedFlowerCount_9_1F4FE5D849688EE7A8AD10AC603CB609` _redflowercount)) (break `/Game/Structures/Struct_PlayerData` (`self.PlayerData`)))
  (bind (_playertransform _blueflowercount_2 _yellowflowercount_2 _redflowercount_2) (break `/Game/Structures/Struct_PlayerData` (`self.PlayerData`)))
  (switch `/Game/Structures/ENUM_FlowerColour` Colour
    (:`NewEnumerator2`
      (`/Engine/EditorBlueprintResources/StandardMacros.IncrementInt` _blueflowercount_2
        (:`  `
          _)))
    (:`NewEnumerator1`
      (`/Engine/EditorBlueprintResources/StandardMacros.IncrementInt` _yellowflowercount_2
        (:`  `
          _)))
    (:`NewEnumerator0`
      (`/Engine/EditorBlueprintResources/StandardMacros.IncrementInt` _redflowercount_2
        (:`  `
          _))))
  (if (>= _blueflowercount 3)
    (if (>= _yellowflowercount 3)
      (if (>= _redflowercount 3)
        (`self.ProgressQuest` "Q_FLOWERS" 1))))
  (return))

(fn `ProgressQuest`
  (params (`Quest ID` :type String) (NewProgressionLevel :type Integer))
  (bind (_playertransform _blueflowercount _yellowflowercount _redflowercount _questprogressmap) (break `/Game/Structures/Struct_PlayerData` (`self.PlayerData`)))
  (`BlueprintMapLibrary.Map_Add` _questprogressmap `Quest ID` (+ NewProgressionLevel (`BlueprintMapLibrary.Map_Find` _questprogressmap `Quest ID`)))
  (return))

(fn `ToggleShield`
  (bind (_name _gender _level _exp _maxhealth _currenthealth _maxmagic _currentmagic _maxarmour _currentarmour _gold _equipment) (break `/Game/Structures/Struct_PlayerStats` (`self.PlayerStats`)))
  (`BlueprintMapLibrary.Map_Add` _equipment "Shield" (not (`BlueprintMapLibrary.Map_Find` _equipment "Shield")))
  (bind _asthird_person_character (cast `/Game/Blueprints/Characters/ThirdPersonCharacter` (`GameplayStatics.GetPlayerPawn` 0)))
  (`/Game/Blueprints/Characters/ThirdPersonCharacter.SetShieldVisibility` _asthird_person_character (`BlueprintMapLibrary.Map_Find` (`.Equipment_40_0265514649013461E03C2AB3F3F476CD` (break `/Game/Structures/Struct_PlayerStats` (`self.PlayerStats`))) "Shield")))